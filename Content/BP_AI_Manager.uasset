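; BP_AI_Manager is an AI spawner that continuously spawns BP_AI3rdPerson characters at BP_AI_SpawnPoint actors in the level.
; On BeginPlay it gathers and shuffles all spawn points, then runs an endless delay loop that spawns one character per SpawnDelay at the next point's transform.
; After every point has been used, it resets the index and reshuffles, giving a random order that covers all points each cycle.
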(event EventBeginPlay
  (bind _outactors (Actor|GetAllActorsOfClass "/Game/BP_AI_SpawnPoint.BP_AI_SpawnPoint_C"))
  (Utilities|Array|Shuffle _outactors)
  (Game|SpawnActorfromClass "/Game/BP_AI3rdPerson.BP_AI3rdPerson_C" (Transformation|GetActorTransform (Utilities|Array|Get(acopy) _outactors (Variables|Default|GetSpawnPointIndex))) "Undefined" 0 0 :!label _label)
  (Math|Integer|IncrementInt (Variables|Default|GetSpawnPointIndex)
    (:%20%20
      (if (>= (Variables|Default|GetSpawnPointIndex) (Utilities|Array|Length _outactors))
        ;[1 1 1] Re-shuffle and reset the index counter.
        (Variables|Default|SetSpawnPointIndex 0)
        (Utilities|Array|Shuffle _outactors))
      (Utilities|FlowControl|Delay (Variables|Default|GetSpawnDelay))
      (goto _label))))

(fn ConstructionScript)